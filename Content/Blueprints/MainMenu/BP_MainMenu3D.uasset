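; BP_MainMenu3D is an actor that hosts the 3D main menu widget and handles view changes away from it.
; On BeginPlay it casts its widget component's widget to WBP_MainMenu3D and passes it the sequence player from the referenced level sequence.
; TransitionTo disables collision on both itself and the given actor, then makes that actor the first player controller's view target through SetViewTargetWithBlend.
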(event `self.ReceiveBeginPlay`
  (bind _aswbp_main_menu_3d (cast `/Game/Blueprints/MainMenu/WBP_MainMenu3D` (`WidgetComponent.GetWidget` (`self.Widget`))))
  (set `/Game/Blueprints/MainMenu/WBP_MainMenu3D.LevelSequencePlayer` (`LevelSequenceActor.SequencePlayer` (`self.LevelSequencePlayerRef`)) _aswbp_main_menu_3d))

(event `TransitionTo`
  (params (NewParam :type "/Game/Blueprints/MainMenu/BP_MainMenu3D Object Reference"))
  (`self.SetActorEnableCollision` false)
  (`self.SetActorEnableCollision` NewParam false)
  (`PlayerController.SetViewTargetWithBlend` (`GameplayStatics.GetPlayerController` 0) NewParam 0.0 "VTBlend_Linear" 0.0 false))

(fn `UserConstructionScript`)