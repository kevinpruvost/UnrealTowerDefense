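; BP_Menu3D is an in-world 3D pause menu actor hosting WBP_Menu3D in a camera-facing widget, linked to a level sequence player.
; Escape, or T in Development builds, toggles it while Playing is set, pausing via near-zero global time dilation.
; Tick eases KwangPlayerRef's music pitch toward a lower paused value, compensating for dilation.
; TransitionTo disables collision on itself and a target, then switches the view to that target.
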(event `Key|T`
  (params (Key :type "Key Structure"))
  (:`Released`
    (if (== (`KismetSystemLibrary.GetBuildConfiguration`) "Development")
      (`self.SetVisible` :!label _label))))

(event `Key|Escape`
  (params (Key :type "Key Structure"))
  (:`Released`
    (goto _label)))

(event `self.ReceiveBeginPlay`
  (set `self.Playing` true)
  (`self.SetVisible`)
  (set `self.Playing` false)
  (`self.SetTickableWhenPaused` true)
  (bind _aswbp_menu_3d (cast `/Game/Blueprints/Menu/WBP_Menu3D` (`WidgetComponent.GetWidget` (`self.Widget`))))
  (set `/Game/Blueprints/Menu/WBP_Menu3D.BP_Menu3DRef` self _aswbp_menu_3d)
  (set `/Game/Blueprints/Menu/WBP_Menu3D.LevelSequencePlayer` (`LevelSequenceActor.SequencePlayer` (`self.LevelSequencePlayerRef`)) _aswbp_menu_3d))

(event `self.ReceiveTick`
  (params (DeltaSeconds :type "Float (single-precision)"))
  (bind _returnvalue (`GameplayStatics.GetGlobalTimeDilation`))
  (bind _widget (`self.Widget`))
  (bind _kwangplayerref (`self.KwangPlayerRef`))
  (bind _returnvalue_2 (/ (`GameplayStatics.GetWorldDeltaSeconds`) _returnvalue))
  (`SceneComponent.K2_SetWorldRotation` _widget (`KismetMathLibrary.Conv_VectorToRotator` (`KismetMathLibrary.GreaterGreater_VectorRotator` (`KismetMathLibrary.Normal` (- (`PlayerCameraManager.GetCameraLocation` (`GameplayStatics.GetPlayerCameraManager` 0)) (`SceneComponent.K2_GetComponentLocation` _widget))))) false false)
  (if (< _returnvalue_2 0.5)
    (bind _pitch (`/Game/Blueprints/KwangPlayerCharacter.GetMusicPitch` _kwangplayerref))
    (`/Game/Blueprints/KwangPlayerCharacter.SetMusicPitch` _kwangplayerref (`KismetMathLibrary.FInterpTo` _pitch (`self.PitchTarget`) _returnvalue_2 (* (`self.Interp Speed`) _returnvalue)))))

(event `TransitionTo`
  (params (NewParam :type "/Game/Blueprints/MainMenu/BP_MainMenu3D Object Reference"))
  (`self.SetActorEnableCollision` false)
  (`self.SetActorEnableCollision` NewParam false)
  (`PlayerController.SetViewTargetWithBlend` (`GameplayStatics.GetPlayerController` 0) NewParam 0.0 "VTBlend_Linear" 0.0 false))

(fn `GetVisible`
  (returns (IsVisible :type Boolean))
  (return (`SceneComponent.IsVisible` (`self.Widget`))))

(fn `SetPause`
  (params (Condition :type Boolean))
  (if Condition
    (`GameplayStatics.SetGlobalTimeDilation` 1e-05)
    (set `self.PitchTarget` 0.2)
    (else
      (`GameplayStatics.SetGlobalTimeDilation` 1.0)
      (set `self.PitchTarget` 1.0))))

(fn `SetVisible`
  (if (`self.Playing`)
    (bind _aswbp_menu_3d (cast `/Game/Blueprints/Menu/WBP_Menu3D` (`WidgetComponent.GetWidget` (`self.Widget`))))
    (bind _enabled (`/Game/Blueprints/Menu/WBP_Menu3D.EnableWidgets` _aswbp_menu_3d))
    (`self.SetPause` _enabled)))

(fn `UserConstructionScript`)