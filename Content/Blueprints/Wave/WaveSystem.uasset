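; Wave manager actor that spawns Narbash enemies at its own location in numbered waves for a game with a castle.
; Starting a wave sets a spawn count that grows with the wave number and spawns immediately, then Tick paces further spawns by SpawnRate, adding health per wave.
; Spawns and deaths update the WaveMenu widget, which reshows its start button once the wave is cleared.
; Reset destroys tracked enemies and restores wave state, menu and castle health.
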(event `self.ReceiveBeginPlay`
  (bind _aswave_menu (cast `/Game/Blueprints/Wave/WaveMenu` (`WidgetComponent.GetWidget` (`self.Widget`))))
  (bind _output_get (set `self.WaveMenuRef` _aswave_menu))
  (set `/Game/Blueprints/Wave/WaveMenu.WaveSystemRef` self _output_get))

(event `self.ReceiveTick`
  (params (DeltaSeconds :type "Float (single-precision)"))
  (if (and (`self.WaveStarted`) (> (`self.RemainingEnemiesToSpawn`) 0))
    (bind _spawnbool (`self.ManageSpawnDelay` DeltaSeconds))
    (if _spawnbool
      (bind _result (`/Engine/EditorBlueprintResources/StandardMacros.IncrementInt` (`self.RemainingEnemies`) :!label _label)
        (:`  `
          (`/Engine/EditorBlueprintResources/StandardMacros.DecrementInt` (`self.RemainingEnemiesToSpawn`)
            (:`  `
              (`self.SpawnEnemy`)
              (`/Game/Blueprints/Wave/WaveMenu.SetEnemiesNb` (`self.WaveMenuRef`) _result))))))))

(event `StartWave`
  (bind _result (`/Engine/EditorBlueprintResources/StandardMacros.IncrementInt` (`self.WaveId`))
    (:`  `
      (set `self.RemainingEnemiesToSpawn` (* _result 5))
      (set `self.SpawnDelay` (`self.SpawnRate`))
      (set `self.WaveStarted` true)
      (`/Game/Blueprints/Wave/WaveMenu.SetWaveNb` (`self.WaveMenuRef`) (`self.WaveId`))
      (goto _label))))

(event `EnemyDie`
  (bind _result (`/Engine/EditorBlueprintResources/StandardMacros.DecrementInt` (`self.RemainingEnemies`))
    (:`  `
      (`/Game/Blueprints/Wave/WaveMenu.SetEnemiesNb` (`self.WaveMenuRef`) _result)
      (if (and (== _result 0) (== (`self.RemainingEnemiesToSpawn`) 0))
        (set `self.WaveStarted` false)
        (`/Game/Blueprints/Wave/WaveMenu.SetStartWaveVisible` (`self.WaveMenuRef`) true)))))

(fn `ManageSpawnDelay`
  (params (Delta :type "Float (double-precision)"))
  (returns (SpawnBool :type Boolean))
  (bind _output_get (set `self.SpawnDelay` (- (`self.SpawnDelay`) Delta)))
  (if (< _output_get 0.0)
    (set `self.SpawnDelay` (`self.SpawnRate`))
    (return true)
    (else
      (return false))))

(fn `Reset`
  (bind _enemiesarray (`self.EnemiesArray`))
  (`/Game/Blueprints/Wave/WaveMenu.ResetMenu` (`self.WaveMenuRef`))
  (set `self.WaveStarted` false)
  (set `self.SpawnDelay` (`self.SpawnRate`))
  (set `self.RemainingEnemies` 0)
  (set `self.RemainingEnemiesToSpawn` 0)
  (set `self.WaveId` 0)
  (for _array_element _enemiesarray
    (`self.K2_DestroyActor` _array_element))
  (`KismetArrayLibrary.Array_Clear` _enemiesarray)
  (`/Game/Blueprints/Castle.ResetHealth` (`self.CastleRef`)))

(fn `SetUIVisible`
  (params (Visible :type Boolean))
  (`/Game/Blueprints/Wave/WaveMenu.SetVisible` (`self.WaveMenuRef`) Visible))

(fn `SpawnEnemy`
  (bind (_returnvalue_location _returnvalue_rotation) (`KismetMathLibrary.BreakTransform` (`SceneComponent.K2_GetComponentToWorld` (`self.DefaultSceneRoot`))))
  (bind _returnvalue (`|SpawnActorFromClass` "/Game/Blueprints/NarbashEnemy.NarbashEnemy_C" (`KismetMathLibrary.MakeTransform` _returnvalue_location _returnvalue_rotation) "Undefined" "OverrideRootScale" null null))
  (`/Game/Blueprints/NarbashEnemy.SetMaxHealth` _returnvalue (+ (`/Game/Blueprints/NarbashEnemy.Health` _returnvalue) (* 20.0 (`self.WaveId`))))
  (set `/Game/Blueprints/NarbashEnemy.WaveMenuRef` self _returnvalue)
  (`KismetArrayLibrary.Array_Add` (`self.EnemiesArray`) _returnvalue))

(fn `UserConstructionScript`)