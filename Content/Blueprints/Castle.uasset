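; Castle actor for a tower defense game that tracks the player base's health and triggers defeat when it runs out.
; On BeginPlay it registers itself in TDGameInstance, sets up a green child-actor health bar and creates a hidden lose-screen widget.
; Damage lowers health and updates the bar, and at zero shows the lose screen and pauses via Menu3DRef.
; ResetHealth restores health to max without refreshing the bar.
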(event `self.ReceiveBeginPlay`
  (bind _healthbarref (`self.HealthBarRef`))
  (bind _astdgame_instance (cast `/Game/Blueprints/TDGameInstance` (`GameplayStatics.GetGameInstance`)))
  (set `/Game/Blueprints/TDGameInstance.CastleRef` self _astdgame_instance)
  (bind _asbp_health_bar (cast `/Game/Blueprints/BP_HealthBar` (`ChildActorComponent.ChildActor` (`self.HealthBar`))))
  (bind _output_get (set `self.HealthBarRef` _asbp_health_bar))
  (`/Game/Blueprints/BP_HealthBar.SetColor` _output_get (make `Color` 0 255 0 255))
  (bind _output_get_2 (set `self.Health` (`self.MaxHealth`)))
  (`/Game/Blueprints/BP_HealthBar.SetMaxHealth` _healthbarref _output_get_2)
  (`/Game/Blueprints/BP_HealthBar.SetHealth` _healthbarref _output_get_2)
  (bind _returnvalue (`|CreateWidget` "/Game/Blueprints/WBP_LoseScreen.WBP_LoseScreen_C"))
  (bind _output_get_3 (set `self.LoseScreen` _returnvalue))
  (`Widget.SetVisibility` _output_get_3 "Collapsed")
  (`UserWidget.AddToViewport` _output_get_3 0))

(fn `Damage`
  (params (Damage :type "Float (double-precision)"))
  (bind _output_get (set `self.Health` (- (`self.Health`) Damage)))
  (`/Game/Blueprints/BP_HealthBar.SetHealth` (`self.HealthBarRef`) _output_get)
  (if (<= _output_get 0.0)
    (`Widget.SetVisibility` (`self.LoseScreen`) "Visible")
    (`/Game/Blueprints/Menu/BP_Menu3D.SetPause` (`self.Menu3DRef`) true)))

(fn `ResetHealth`
  (set `self.Health` (`self.MaxHealth`)))

(fn `UserConstructionScript`)