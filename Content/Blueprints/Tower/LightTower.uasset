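; LightTower is a tower Blueprint that fires LightMissile projectiles, although it registers itself under the name "Fire Tower".
; On BeginPlay it passes per-level costs, damages and fire rates, plus a range radius, to the inherited Instantiate.
; Fire plays a sound, spawns a scaled-down missile at an offset relative to the tower's transform, and sets its damage from GetDamage.
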(event `self.ReceiveBeginPlay`
  (`parent.ReceiveBeginPlay`)
  (`self.Instantiate` "Fire Tower" (`|MakeArray` 750 1000 1500 2000) (`|MakeArray` 20 25 30 40 50) (`|MakeArray` 1.0 0.5 0.333333 0.25 0.2) 1000))

(fn `Fire`
  (`GameplayStatics.PlaySoundAtLocation` "/Game/Sound/Se_effect_fast.Se_effect_fast" (`self.K2_GetActorLocation`) (struct) 1.0 1.0 0.0 null null null null)
  (bind _returnvalue (`|SpawnActorFromClass` "/Game/Blueprints/Tower/LightMissile.LightMissile_C" (`KismetMathLibrary.ComposeTransforms` (`KismetMathLibrary.MakeTransform` (100.0 0.0 100.0) (struct) (0.3 0.3 0.3)) (`self.GetTransform`)) "AlwaysSpawn" "OverrideRootScale" null self))
  (bind _damage (`self.GetDamage`))
  (`/Game/Blueprints/Tower/BaseMissile.SetDamage` _returnvalue (`KismetMathLibrary.Conv_IntToDouble` _damage)))

(fn `UserConstructionScript`
  (`parent.UserConstructionScript`))