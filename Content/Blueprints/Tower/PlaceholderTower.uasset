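; PlaceholderTower is a tower placeholder actor that shows a purchase interface while the Kwang player character overlaps it.
; On BeginPlay it casts its widget component's widget to InterfacePurchase and sets itself as that widget's Parent.
; Begin and end overlap events call TriggerInterface, which toggles the widget between SelfHitTestInvisible and Collapsed.
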(event `self.ReceiveBeginPlay`
  (bind _asinterface_purchase (cast `/Game/Blueprints/Tower/InterfacePurchase` (`WidgetComponent.GetWidget` (`self.Widget`))))
  (set `/Game/Blueprints/Tower/InterfacePurchase.Parent` self _asinterface_purchase))

(event `self.ReceiveActorBeginOverlap`
  (params (OtherActor :type "Actor Object Reference"))
  (cast `/Game/Blueprints/KwangPlayerCharacter` OtherActor)
  (`self.TriggerInterface` true))

(event `self.ReceiveActorEndOverlap`
  (params (OtherActor :type "Actor Object Reference"))
  (cast `/Game/Blueprints/KwangPlayerCharacter` OtherActor)
  (`self.TriggerInterface` false))

(fn `TriggerInterface`
  (params (Display :type Boolean))
  (bind _returnvalue (`WidgetComponent.GetWidget` (`self.Widget`)))
  (if (`KismetSystemLibrary.IsValid` _returnvalue)
    (if Display
      (`Widget.SetVisibility` _returnvalue "SelfHitTestInvisible")
      (else
        (`Widget.SetVisibility` _returnvalue "Collapsed")))))

(fn `UserConstructionScript`)