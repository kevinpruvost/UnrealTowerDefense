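; BaseMissile is a tower projectile base that damages NarbashEnemy actors it overlaps and destroys itself after three seconds.
; On BeginPlay it binds the overlap handler to a child box component, which applies Damage with sound, then calls AdditionalInteractions, an empty hook.
; Hits do not destroy the missile.
; SetDamage assigns only negative values and returns false on both branches.
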(event `self.ReceiveBeginPlay`
  (for _array_element (`SceneComponent.GetChildrenComponents` (`self.DefaultSceneRoot`) true)
    (bind _asbox_collision (cast `BoxComponent` _array_element))
    (add `PrimitiveComponent.OnComponentBeginOverlap` _asbox_collision (delegate `OnComponentBeginOverlap_Missile`))
    (break))
  (`KismetSystemLibrary.Delay` 3.0)
  (`self.K2_DestroyActor`))

(event `OnComponentBeginOverlap_Missile`
  (params (OverlappedComponent :type "PrimitiveComponent Object Reference") (OtherActor :type "Actor Object Reference") (OtherComp :type "PrimitiveComponent Object Reference") (OtherBodyIndex :type Integer) (bFromSweep :type Boolean) (SweepResult :type "HitResult Structure (by ref)"))
  (bind _asnarbash_enemy (cast `/Game/Blueprints/NarbashEnemy` OtherActor))
  (`/Game/Blueprints/NarbashEnemy.Damage` _asnarbash_enemy (`self.Damage`) true)
  (`self.AdditionalInteractions` _asnarbash_enemy))

(fn `AdditionalInteractions`
  (params (Enemy :type "/Game/Blueprints/NarbashEnemy Object Reference (by ref)")))

(fn `SetDamage`
  (params (Damage :type "Float (double-precision)" :default 0.0))
  (returns (Success :type Boolean))
  (if (>= (`self.Damage`) 0.0)
    (return false)
    (else
      (set `self.Damage` Damage)
      (return false))))

(fn `UserConstructionScript`)