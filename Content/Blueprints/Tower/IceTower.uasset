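; Ice tower Blueprint that fires ice missiles, built on a parent tower class.
; On BeginPlay it runs the parent's setup, then calls Instantiate with its name, upgrade costs, per-level damage and fire rates, and range.
; Fire plays an ice sound, spawns a half-scale IceMissile at an offset relative to the tower's transform, and passes it the tower's current damage.
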(event `self.ReceiveBeginPlay`
  (`parent.ReceiveBeginPlay`)
  (`self.Instantiate` "Ice Tower" (`|MakeArray` 750 1000 1250 1500) (`|MakeArray` 20 25 30 35 40) (`|MakeArray` 2.0 1.8 1.5 1.2 0.8) 1000))

(fn `Fire`
  (`GameplayStatics.PlaySoundAtLocation` "/Game/Sound/Se_effect_ice.Se_effect_ice" (`self.K2_GetActorLocation`) (struct) 1.0 1.0 0.0 null null null null)
  (bind _returnvalue (`|SpawnActorFromClass` "/Game/Blueprints/Tower/IceMissile.IceMissile_C" (`KismetMathLibrary.ComposeTransforms` (`KismetMathLibrary.MakeTransform` (100.0 0.0 100.0) (struct) (0.5 0.5 0.5)) (`self.GetTransform`)) "Undefined" "OverrideRootScale" null self))
  (bind _damage (`self.GetDamage`))
  (`/Game/Blueprints/Tower/BaseMissile.SetDamage` _returnvalue (`KismetMathLibrary.Conv_IntToDouble` _damage)))

(fn `UserConstructionScript`)