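; Base tower-defense tower that targets Narbash enemies in range, with an empty Fire function as the attack hook.
; Each tick it picks an enemy unblocked by static geometry, yaws toward it, and checks alignment and fire-rate timer before firing.
; Instantiate sets per-level stats, range and the widget, which shows while the Kwang player is near.
; LevelUp spends game-instance money to advance the level.
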(event `self.ReceiveTick`
  (params (DeltaSeconds :type "Float (single-precision)"))
  (bind _res (`self.SelectTarget` DeltaSeconds))
  (bind _res_2 (`self.ShouldFire` DeltaSeconds _res))
  (if _res_2
    (`self.Fire`)))

(event `self.Range.OnComponentBeginOverlap`
  (params (OverlappedComponent :type "PrimitiveComponent Object Reference") (OtherActor :type "Actor Object Reference") (OtherComp :type "PrimitiveComponent Object Reference") (OtherBodyIndex :type Integer) (bFromSweep :type Boolean) (SweepResult :type "HitResult Structure (by ref)"))
  (bind _asnarbash_enemy (cast `/Game/Blueprints/NarbashEnemy` OtherActor))
  (`KismetArrayLibrary.Array_Add` (`self.Enemies`) _asnarbash_enemy))

(event `self.Range.OnComponentEndOverlap`
  (params (OverlappedComponent :type "PrimitiveComponent Object Reference") (OtherActor :type "Actor Object Reference") (OtherComp :type "PrimitiveComponent Object Reference") (OtherBodyIndex :type Integer))
  (bind _asnarbash_enemy (cast `/Game/Blueprints/NarbashEnemy` OtherActor))
  (`KismetArrayLibrary.Array_RemoveItem` (`self.Enemies`) _asnarbash_enemy))

(event `self.PDetector.OnComponentBeginOverlap`
  (params (OverlappedComponent :type "PrimitiveComponent Object Reference") (OtherActor :type "Actor Object Reference") (OtherComp :type "PrimitiveComponent Object Reference") (OtherBodyIndex :type Integer) (bFromSweep :type Boolean) (SweepResult :type "HitResult Structure (by ref)"))
  (cast `/Game/Blueprints/KwangPlayerCharacter` OtherActor)
  (`Widget.SetVisibility` (`WidgetComponent.GetWidget` (`self.Widget`)) "SelfHitTestInvisible"))

(event `self.PDetector.OnComponentEndOverlap`
  (params (OverlappedComponent :type "PrimitiveComponent Object Reference") (OtherActor :type "Actor Object Reference") (OtherComp :type "PrimitiveComponent Object Reference") (OtherBodyIndex :type Integer))
  (cast `/Game/Blueprints/KwangPlayerCharacter` OtherActor)
  (`Widget.SetVisibility` (`WidgetComponent.GetWidget` (`self.Widget`)) "Collapsed"))

(fn `Fire`)

(fn `GetCurrentLevel`
  (returns (Level :type Integer))
  (return (`self.Level`)))

(fn `GetDamage`
  (returns (Damage :type Integer))
  (if (`self.isReady`)
    (return (`|GetArrayItem` (`self.Damages`) (- (`self.Level`) 1)))
    (else
      (return 0))))

(fn `GetFireRate`
  (returns (FireRate :type "Float (double-precision)"))
  (if (`self.isReady`)
    (return (`|GetArrayItem` (`self.FireRates`) (- (`self.Level`) 1)))
    (else
      (return 0.0))))

(fn `GetNextLevelCost`
  (returns (Cost :type Integer))
  (bind _level (`self.Level`))
  (bind _costs (`self.Costs`))
  (if (> _level (`KismetArrayLibrary.Array_Length` _costs))
    (return 0)
    (else
      (return (`|GetArrayItem` _costs (- _level 1))))))

(fn `GetRange`
  (returns (Range :type Integer))
  (return (`KismetMathLibrary.FTrunc` (`SphereComponent.GetScaledSphereRadius` (`self.Range`)))))

(fn `Instantiate`
  (params (Name :type String) (LevelCosts :type "Array of Integer") (Damages :type "Array of Integer") (FireRates :type "Array of Float (double-precision)") (RangeRadius :type Integer))
  (returns (Done :type Boolean))
  (bind _returnvalue (`KismetArrayLibrary.Array_Length` Damages))
  (bind _returnvalue_2 (`KismetArrayLibrary.Array_Length` FireRates))
  (if (or (!= (+ (`KismetArrayLibrary.Array_Length` LevelCosts) 1) _returnvalue) (!= _returnvalue _returnvalue_2))
    (return (`self.isReady`))
    (else
      (set `self.Costs` LevelCosts)
      (set `self.Damages` Damages)
      (set `self.FireRates` FireRates)
      (set `self.Level` (`KismetMathLibrary.Min` _returnvalue_2 (`self.Level`)))
      (`SphereComponent.SetSphereRadius` (`self.Range`) (`KismetMathLibrary.Conv_IntToDouble` RangeRadius) true)
      (bind _output_get (set `self.isReady` true))
      (bind _asinterface_tower (cast `/Game/Blueprints/Tower/InterfaceTower` (`WidgetComponent.GetWidget` (`self.Widget`))))
      (`/Game/Blueprints/Tower/InterfaceTower.Instantiate` _asinterface_tower self Name)
      (return _output_get))))

(fn `LevelUp`
  (returns (Success :type Boolean))
  (bind _level (`self.Level`))
  (bind _costs (`self.Costs`))
  (bind _astdgame_instance (cast `/Game/Blueprints/TDGameInstance` (`GameplayStatics.GetGameInstance`)))
  (bind _returnvalue (- (`/Game/Blueprints/TDGameInstance.Money` _astdgame_instance) (`|GetArrayItem` _costs (- _level 1))))
  (if (or (> _level (`KismetArrayLibrary.Array_Length` _costs)) (< _returnvalue 0))
    (return false)
    (else
      (set `/Game/Blueprints/TDGameInstance.Money` _returnvalue _astdgame_instance)
      (`/Engine/EditorBlueprintResources/StandardMacros.IncrementInt` _level
        (:`  `
          (return true))))))

(fn `SelectTarget`
  (params (DeltaTime :type "Float (double-precision)"))
  (returns (Res :type Boolean))
  (locals (Rot :type "Float (single-precision)" :default 0.0) (Target :type "/Game/Blueprints/NarbashEnemy Object Reference"))
  (bind _returnvalue (* DeltaTime 90.0))
  (bind _rot (`local.Rot`))
  (bind _yaw (.yaw (`self.K2_GetActorRotation`)))
  (bind _returnvalue_2 (`KismetMathLibrary.FMin` _rot _returnvalue))
  (bind _returnvalue_3 (`KismetMathLibrary.FMax` _rot _returnvalue))
  (for _array_element (`self.Enemies`)
    (bind (_outhit _returnvalue_4) (`KismetSystemLibrary.LineTraceSingleForObjects` (+ (`self.K2_GetActorLocation`) (50.0 0.0 50.0)) (`self.K2_GetActorLocation` _array_element) (`|MakeArray` (enumliteral `EObjectTypeQuery` "ObjectTypeQuery1"))))
    (if (not _returnvalue_4)
      (set `local.Target` _array_element)
      (break)))
  (`/Engine/EditorBlueprintResources/StandardMacros.IsValid` (`local.Target`)
    (:`Is Valid`
      (bind _output_get (set `local.Rot` (.yaw (`KismetMathLibrary.FindRelativeLookAtRotation` (`self.GetTransform`) (`self.K2_GetActorLocation` (`local.Target`))))))
      (if (> _output_get 0.0)
        (`self.K2_SetActorRotation` (`KismetMathLibrary.MakeRotator` 0.0 0.0 (+ _returnvalue_2 _yaw)))
        (return (== _rot _returnvalue_2))
        (else
          (`self.K2_SetActorRotation` (`KismetMathLibrary.MakeRotator` 0.0 0.0 (- _yaw _returnvalue_3)))
          (return (== (`local.Rot`) _returnvalue_3)))))
    (:`Is Not Valid`
      (return false))))

(fn `ShouldFire`
  (params (DeltaTime :type "Float (double-precision)") (isAligned :type Boolean))
  (returns (Res :type Boolean))
  (bind _returnvalue (+ DeltaTime (`self.LastFire`)))
  (bind _output (`|GetArrayItem` (`self.FireRates`) (- (`self.Level`) 1)))
  (bind _output_get (set `self.LastFire` _returnvalue))
  (if (or (not isAligned) (not (`self.isReady`)))
    (return false)
    (else
      (set `self.LastFire` (mod _output_get _output))
      (return (>= _returnvalue _output)))))

(fn `UserConstructionScript`)